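; Third-person player character with Enhanced Input movement and look, a jetpack and a charged propulsion boost.
; Holding jump applies upward impulses that drain jetpack charge, enabled after a short delay following the jump.
; Holding Propulse builds capped power, and releasing it launches the character up and forward, spending a propulse charge.
; Tick restores both charge pools to their BeginPlay values and clears the jumping flag whenever the character is grounded.
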(event Input|EnhancedActionEvents|EnhancedInputActionIA_Move
  (params (ActionValue :type Vector%202D%20Structure) (ElapsedSeconds :type Float%20%28double-precision%29) (TriggeredSeconds :type Float%20%28double-precision%29) (InputAction :type Input%20Action%20Object%20Reference :default "/Game/Projet/Inputs/Actions/IA_Move.IA_Move"))
  (Pawn|Input|AddMovementInput (Transformation|GetActorRightVector) (.x ActionValue) false)
  (Pawn|Input|AddMovementInput (Transformation|GetActorForwardVector) (.y ActionValue) false))

(event Input|EnhancedActionEvents|EnhancedInputActionIA_Look
  (params (ActionValue :type Vector%202D%20Structure) (ElapsedSeconds :type Float%20%28double-precision%29) (TriggeredSeconds :type Float%20%28double-precision%29) (InputAction :type Input%20Action%20Object%20Reference :default "/Game/Projet/Inputs/Actions/IA_Look.IA_Look"))
  (Pawn|Input|AddControllerYawInput (.x ActionValue))
  (Pawn|Input|AddControllerPitchInput (.y ActionValue)))

(event Input|EnhancedActionEvents|EnhancedInputActionIA_Jump
  (params (ActionValue :type Boolean) (ElapsedSeconds :type Float%20%28double-precision%29) (TriggeredSeconds :type Float%20%28double-precision%29) (InputAction :type Input%20Action%20Object%20Reference :default "/Game/Projet/Inputs/Actions/IA_Jump.IA_Jump"))
  (:Triggered
    (if (Variables|Default|GetIsjumping)
      (if (> (Variables|Default|GetJetpackcharge) 0.0)
        (Physics|AddImpulse (Variables|Character|GetCharacterMovement) (* (Math|Vector|VectorUp) "0.000000,0.000000,700.000000") false)
        (bind _result (Math|Float|DecrementFloat (Variables|Default|GetJetpackcharge))
          (:%20%20
            (bind _output_get (Variables|Default|SetJetpackcharge _result))
            (Development|PrintString (Utilities|String|ToString(Float) _output_get)))))))
  (:Started
    (Character|Jump)
    (Utilities|FlowControl|Delay 0.25)
    (Variables|Default|SetIsjumping true))
  (:Completed
    (Character|StopJumping)))

(event Input|EnhancedActionEvents|EnhancedInputActionIA_Propulse
  (params (ActionValue :type Boolean) (ElapsedSeconds :type Float%20%28double-precision%29) (TriggeredSeconds :type Float%20%28double-precision%29) (InputAction :type Input%20Action%20Object%20Reference :default "/Game/Projet/Inputs/Actions/IA_Propulse.IA_Propulse"))
  (:Triggered
    ;[1 1 1] Charge du boost propulseur
    (if (< (Variables|Default|GetPropulseParam) 1.5e+02)
      (bind _result (Math|Float|IncrementFloat (Variables|Default|GetPropulseParam))
        (:%20%20
          (bind _output_get (Variables|Default|SetPropulseParam _result))
          (Development|PrintString (Utilities|String|ToString(Float) _output_get))))))
  (:Completed
    ;[1 1 1] Propulsion
    (if (> (Variables|Default|GetPropulsecharge) 0)
      (Character|LaunchCharacter (+ (* (Math|Vector|VectorUp) "0.000000,0.000000,10.000000" (Variables|Default|GetPropulseParam)) (* (Math|Vector|GetForwardVector (Variables|Collision|GetCapsuleComponent)) 2e+02)) true true)
      (Variables|Default|SetPropulseParam 0.0)
      (bind _result_2 (Math|Integer|DecrementInt (Variables|Default|GetPropulsecharge))
        (:%20%20
          (Variables|Default|SetPropulsecharge _result_2))))))

(event EventTick
  (params (DeltaSeconds :type Float%20%28single-precision%29))
  (if (AI|Components|NavMovement|IsMovingonGround (Variables|Character|GetCharacterMovement))
    (Variables|Default|SetPropulsecharge (Variables|Default|GetBasePropulseCharge))
    (Variables|Default|SetJetpackcharge (Variables|Default|GetBaseJetpackCharge))
    (Variables|Default|SetIsjumping false)))

(event EventBeginPlay
  (Variables|Default|SetBaseJetpackCharge (Variables|Default|GetJetpackcharge))
  (Variables|Default|SetBasePropulseCharge (Variables|Default|GetPropulsecharge)))

(fn ConstructionScript)